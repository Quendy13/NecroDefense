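; BP_Minion_Parent is the base minion Blueprint, driven by an AI controller running the BT_Minion behavior tree.
; On BeginPlay it starts the tree, caches the blackboard and stores the BP_ThirdPersonCharacter as PlayerRef.
; AI perception updates write a detected BP_Enemy_Parent into EnnemyRef only while that key holds no valid object, so the minion keeps its current target.
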(event `self.ReceiveBeginPlay`
  (`|ExecutionSequence`
    (:`then_0`
      (bind _asaicontroller (cast `AIController` (`self.GetController`)))
      (`AIController.RunBehaviorTree` _asaicontroller "/Game/Blueprints/Minions/AI/BT_Minion.BT_Minion")
      (set `self.BlackboardRef` (`AIBlueprintHelperLibrary.GetBlackboard` (`self.GetController`)))
      (bind _returnvalue (`GameplayStatics.GetActorOfClass` "/Game/Blueprints/Player/BP_ThirdPersonCharacter.BP_ThirdPersonCharacter_C"))
      (`BlackboardComponent.SetValueAsObject` (`self.BlackboardRef`) "PlayerRef" _returnvalue))))

(event `self.AIPerception.OnTargetPerceptionUpdated`
  (params (Actor :type "Actor Object Reference") (Stimulus :type "AIStimulus Structure"))
  (bind _blackboardref (`self.BlackboardRef`))
  (bind _asbp_ennemy_parent (cast `/Game/Blueprints/Enemies/BP_Enemy_Parent` Actor))
  (`/Engine/EditorBlueprintResources/StandardMacros.IsValid` (`BlackboardComponent.GetValueAsObject` _blackboardref "EnnemyRef")
    (:`Is Not Valid`
      (`BlackboardComponent.SetValueAsObject` _blackboardref "EnnemyRef" _asbp_ennemy_parent))))

(fn `UserConstructionScript`)